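; bpSomethingNotCar is a drivable vehicle with axis inputs for throttle and scaled-down steering, fed to its VehicleMovement component.
; Space bar acts as a brake: while held, a Tick-driven gate forces throttle to zero.
; The same press plays a deceleration timeline that multiplies the mesh's current linear velocity by a curve fraction on each update, overriding physics velocity directly until release stops it.
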(event `self.ReceiveTick`
  (params (DeltaSeconds :type "Float (single-precision)"))
  (set `self.DeltaSeconds` DeltaSeconds)
  (`/Engine/EditorBlueprintResources/StandardMacros.Gate` true :!label _label
    (:`Exit`
      (`WheeledVehicleMovementComponent.SetThrottleInput` (`self.VehicleMovement`) 0.0))))

(event `Key|SpaceBar`
  (params (Key :type "Key Structure"))
  (:`Pressed`
    (goto _label :!via `Open`))
  (:`Released`
    (goto _label :!via `Close`)))

(event `InputAxis|GasPedal`
  (params (AxisValue :type "Float (single-precision)"))
  (`WheeledVehicleMovementComponent.SetThrottleInput` (`self.VehicleMovement`) AxisValue))

(event `InputAxis|Steering`
  (params (AxisValue :type "Float (single-precision)"))
  (`WheeledVehicleMovementComponent.SetSteeringInput` (`self.VehicleMovement`) (/ AxisValue 10.0)))

(event `Key|SpaceBar`
  (params (Key :type "Key Structure"))
  (:`Pressed`
    (bind (_direction _velocityfraction) (`Timeline|DecelerationTimeline` :!via `PlayFromStart` :!label _label_2)
      (:`Update`
        (bind _returnvalue (`PrimitiveComponent.GetPhysicsLinearVelocity` (`self.Mesh`) "None"))
        (`PrimitiveComponent.SetAllPhysicsLinearVelocity` (`self.Mesh`) (* _returnvalue _velocityfraction) false))))
  (:`Released`
    (goto _label_2 :!via `Stop`)))

(fn `UserConstructionScript`)